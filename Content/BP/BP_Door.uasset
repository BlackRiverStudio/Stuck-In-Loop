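; BP_Door is an automatic sliding door that opens when the player character enters its trigger Box and closes when they leave.
; Both overlap events ignore actors other than player 0's character, then drive the SlidingDoor timeline, which lerps the Cube's relative X location to slide it.
; Opening always plays from the start and closing reverses from the end, so an interrupted slide jumps rather than resuming.
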(event OnComponentBeginOverlap(Box)
  (params (OverlappedComponent :type Primitive%20Component%20Object%20Reference) (OtherActor :type Actor%20Object%20Reference) (OtherComp :type Primitive%20Component%20Object%20Reference) (OtherBodyIndex :type Integer) (bFromSweep :type Boolean) (SweepResult :type Hit%20Result%20Structure%20%28by%20ref%29))
  ;[1 1 1] First Person Character - When entering trigger, door slides open automatically. When player leaves trigger, door closes automatically
  (if (== (Game|GetPlayerCharacter 0) OtherActor)
    (bind _doortrack (Timeline|SlidingDoor PlayFromStart)
      (:Update
        (Transformation|SetRelativeLocation (Variables|Default|GetCube) (Math|Vector|MakeVector (Math|Float|Lerp 0.0 -1.7e+02 _doortrack) 0.0 0.0) false false)))))

(event OnComponentEndOverlap(Box)
  (params (OverlappedComponent :type Primitive%20Component%20Object%20Reference) (OtherActor :type Actor%20Object%20Reference) (OtherComp :type Primitive%20Component%20Object%20Reference) (OtherBodyIndex :type Integer))
  ;[1 1 1] First Person Character - When entering trigger, door slides open automatically. When player leaves trigger, door closes automatically
  (if (== (Game|GetPlayerCharacter 0) OtherActor)
    (bind _doortrack (Timeline|SlidingDoor ReverseFromEnd)
      (:Update
        (Transformation|SetRelativeLocation (Variables|Default|GetCube) (Math|Vector|MakeVector (Math|Float|Lerp 0.0 -1.7e+02 _doortrack) 0.0 0.0) false false)))))

(fn ConstructionScript)