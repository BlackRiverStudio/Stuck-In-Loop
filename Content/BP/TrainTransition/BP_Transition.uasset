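; BP_Transition is a one-way trigger plane that teleports the first-person player to a linked transition actor, either looping or progressing.
; Each tick, while the player overlaps PlayerDetection, a dot-product and line-plane test detects the camera crossing front to back.
; A key check picks ProgressPortal or LoopPortal, but is stubbed false, so it always loops.
; Teleporting targets the chosen portal's Target location; render-target portal view code is disconnected.
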(event EventBeginPlay
  (bind _asbp_first_person_character (Utilities|Casting|CastToBP_FirstPersonCharacter (Game|GetPlayerCharacter 0)))
  (Variables|Default|SetAs%20BP%20First%20Person%20Character _asbp_first_person_character))

(event Collision|EventActorBeginOverlap
  (params (OtherActor :type Actor%20Object%20Reference)))

(event EventTick
  (params (DeltaSeconds :type Float%20%28single-precision%29))
  (CallFunction|CheckShouldTeleport))

(fn ConstructionScript)

(fn CheckViewPortSize
  (bind _returnvalue (Viewport|GetViewportSize))
  (bind _returnvalue_2 (Viewport|GetViewportSize))
  (bind _portal_rt (Variables|Default|GetPORTAL_RT))
  (bind (_x _y) (Math|Vector2D|BreakVector2D _returnvalue))
  (bind (_x_2 _y_2) (Math|Vector2D|BreakVector2D _returnvalue_2))
  (Utilities|IsValid (Variables|Default|GetPORTAL_RT)
    (:Is%20Valid
      (if (not (and (== _x (Variables|/Script/Engine.TextureRenderTarget2D|GetSizeX _portal_rt)) (== _y (Variables|/Script/Engine.TextureRenderTarget2D|GetSizeY _portal_rt))))
        (Development|PrintString "Rezize")
        (Rendering|ResizeRenderTarget2D (Variables|Default|GetPORTAL_RT) (Math|Float|Truncate _x_2) (Math|Float|Truncate _y_2))))
    (:Is%20Not%20Valid
      (Development|PrintString "something broke"))))

(fn CheckShouldTeleport
  (Utilities|IsValid (Utilities|Array|Get(acopy) (Collision|GetOverlappingActors (Variables|Default|GetPlayerDetection) "/Game/FirstPerson/Blueprints/BP_FirstPersonCharacter.BP_FirstPersonCharacter_C" :!class /Script/Engine.PrimitiveComponent))
    (:Is%20Valid
      (bind _asbp_first_person_character (Utilities|Casting|CastToBP_FirstPersonCharacter (Game|GetPlayerCharacter 0)))
      (bind _bresult (CallFunction|IsPointCrossingPortal (Transformation|GetWorldLocation (Variables|/Script/StuckInLoop.StuckInLoopCharacter|GetFirstPersonCameraComponent _asbp_first_person_character)) (Transformation|GetActorLocation) (Math|Vector|GetForwardVector (Variables|Default|GetforwardDirection))))
      (if _bresult
        (Development|PrintString "whoop!")
        (bind _bhasobject_ (CallFunction|CheckAmHoldingKey))
        (if _bhasobject_
          (Variables|Default|SetLinkedPortal (Variables|Default|GetProgressPortal))
          (else
            (Variables|Default|SetLinkedPortal (Variables|Default|GetLoopPortal))))
        (CallFunction|TeleportCharacter (Variables|Default|GetLinkedPortal))))))

(fn IsPointCrossingPortal
  (params (Point :type Vector) (PortalLocation :type Vector) (PortalNormal :type Vector))
  (LocalVariables|SetbIsInFront (>= (Math|Vector|DotProduct PortalNormal (- Point PortalLocation)) 0.0))
  (LocalVariables|SetbIsCrossing (Math|Boolean|ANDBoolean (.ReturnValue (Class|KismetMathLibrary|LinePlaneIntersection (Variables|Default|GetLastPosition) Point (Class|KismetMathLibrary|MakePlanefromPointandNormal PortalLocation PortalNormal))) (not (LocalVariables|GetbIsInFront)) (Variables|Default|GetbLastInFront)))
  (Variables|Default|SetbLastInFront (LocalVariables|GetbIsInFront))
  (Variables|Default|SetLastPosition Point)
  (return (LocalVariables|GetbIsCrossing)))

(fn TeleportCharacter
  (params (GoalPortal :type BP%20Transition%20Object%20Reference))
  (Transformation|SetActorTransform (Variables|Default|GetAs%20BP%20First%20Person%20Character) (Math|Transform|MakeTransform (Transformation|GetWorldLocation (Variables|BP_Transition_C|GetTarget GoalPortal)) "0, 0, 0" "1.000000,1.000000,1.000000") false true))

(fn CheckAmHoldingKey
  (Development|PrintString "yueh nuh not this, chief")
  (return false))