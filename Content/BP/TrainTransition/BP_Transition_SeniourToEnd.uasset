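; Portal actor for the senior-to-end train transition that either ends the loop or sends the player back.
; When the first-person character's camera crosses the portal plane within the detection volume, CheckShouldTeleport branches on the held object.
; Empty hands load L_AfterlifeFog as a level instance; holding any object teleports the player to LoopPortal.
; Despite its name, CheckAmHoldingKey returns true when nothing is held.
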(event EventBeginPlay
  (|CallParentFunction) ; This node is disabled and will not be called.\nDrag off pins to build functionality.
)

(event Collision|EventActorBeginOverlap
  (params (OtherActor :type Actor%20Object%20Reference))
  (|CallParentFunction OtherActor) ; This node is disabled and will not be called.\nDrag off pins to build functionality.
)

(event EventTick
  (params (DeltaSeconds :type Float%20%28single-precision%29))
  (|CallParentFunction DeltaSeconds) ; This node is disabled and will not be called.\nDrag off pins to build functionality.
)

(fn ConstructionScript
  (|CallParentFunction))

(fn CheckAmHoldingKey
  (bind _asbp_first_person_character (Utilities|Casting|CastToBP_FirstPersonCharacter (Game|GetPlayerCharacter 0))
    (:then
      (Utilities|IsValid (Variables|/Game/FirstPerson/Blueprints/BP_FirstPersonCharacter.BP_FirstPersonCharacter_C|GetHeld%20Object _asbp_first_person_character)
        (:Is%20Valid
          (return false))
        (:Is%20Not%20Valid
          (return true))))
    (:CastFailed
      (return false))))

(fn CheckShouldTeleport
  (Utilities|IsValid (Utilities|Array|Get(acopy) (Collision|GetOverlappingActors (Variables|Default|GetPlayerDetection) "/Game/FirstPerson/Blueprints/BP_FirstPersonCharacter.BP_FirstPersonCharacter_C" :!class /Script/Engine.PrimitiveComponent))
    (:Is%20Valid
      (bind _asbp_first_person_character (Utilities|Casting|CastToBP_FirstPersonCharacter (Game|GetPlayerCharacter 0)))
      (bind _bresult (CallFunction|IsPointCrossingPortal (Transformation|GetWorldLocation (Variables|/Script/StuckInLoop.StuckInLoopCharacter|GetFirstPersonCameraComponent _asbp_first_person_character)) (Transformation|GetActorLocation) (Math|Vector|GetForwardVector (Variables|Default|GetforwardDirection))))
      (if _bresult
        (Development|PrintString "whoop!")
        (bind _bhasobject_ (CallFunction|CheckAmHoldingKey))
        (if _bhasobject_
          (Class|LevelStreamingDynamic|LoadLevelInstancebySoftObjectPtr "/Game/FirstPerson/Maps/L_AfterlifeFog.L_AfterlifeFog" "0, 0, 0" "0, 0, 0" "" 0 false)
          (else
            (Variables|Default|SetLinkedPortal (Variables|Default|GetLoopPortal))
            (CallFunction|TeleportCharacter (Variables|Default|GetLinkedPortal))))))))