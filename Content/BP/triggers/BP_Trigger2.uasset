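; BP_Trigger2 is a trigger volume that shows a train message on screen while the player character is inside its Box.
; On begin overlap by player 0's character, it creates a WBP_TrainMessage3 widget and adds it to the viewport.
; On end overlap, it creates a WBP_TrainMessage1 without displaying it, then calls RemoveAllWidgets, clearing every viewport widget rather than just its own.
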(event OnComponentBeginOverlap(Box)
  (params (OverlappedComponent :type Primitive%20Component%20Object%20Reference) (OtherActor :type Actor%20Object%20Reference) (OtherComp :type Primitive%20Component%20Object%20Reference) (OtherBodyIndex :type Integer) (bFromSweep :type Boolean) (SweepResult :type Hit%20Result%20Structure%20%28by%20ref%29))
  (if (== (Game|GetPlayerCharacter 0) OtherActor)
    (bind _returnvalue (UserInterface|CreateWidget "/Game/UI/WBP_TrainMessage3.WBP_TrainMessage3_C"))
    (UserInterface|Viewport|AddtoViewport _returnvalue 0)))

(event OnComponentEndOverlap(Box)
  (params (OverlappedComponent :type Primitive%20Component%20Object%20Reference) (OtherActor :type Actor%20Object%20Reference) (OtherComp :type Primitive%20Component%20Object%20Reference) (OtherBodyIndex :type Integer))
  (if (== (Game|GetPlayerCharacter 0) OtherActor)
    (UserInterface|CreateWidget "/Game/UI/WBP_TrainMessage1.WBP_TrainMessage1_C")
    (Viewport|RemoveAllWidgets)))

(event EventBeginPlay)

(event Collision|EventActorBeginOverlap
  (params (OtherActor :type Actor%20Object%20Reference)))

(event EventTick
  (params (DeltaSeconds :type Float%20%28single-precision%29)))

(fn ConstructionScript)